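; An enemy AI controller, themed as a loan shark, that chases the player.
; On BeginPlay a one-second looping timer calls DIVIDA-COM-AGIOTA, which reissues an AI move toward the player pawn.
; The Paredão and CobraPão events stop movement but leave the timer running.
; The startAI event only prints the distance between the player and the controlled pawn.
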(event Custom|DIVIDA-COM-AGIOTA
  ;[1 1 1] É o Seguinte:
  (AI|AIMoveTo 0 "0, 0, 0" (Game|Player|GetPlayerPawn 0) 5.0 false))

(event Custom|Paredão
  ;[1 1 1] Parado
  (AI|Navigation|StopMovement))

(event Custom|Cobra%20Pão
  ;[1 1 1] Parado
  (AI|Navigation|StopMovement))

(event Custom|startAI
  (params (FunctionName :type String))
  ;[1 1 1] Dívida
  (bind _output_get (Variables|Default|SetDISTANCE (Transformation|GetDistanceTo (Game|Player|GetPlayerPawn 0) (Pawn|GetControlledPawn))))
  (Development|PrintString (Utilities|String|ToString(Float) _output_get)))

(event EventBeginPlay
  ;[1 1 1] Dívida
  (Utilities|Time|SetTimerbyFunctionName 0 "DIVIDA-COM-AGIOTA" 1.0 true))

(fn ConstructionScript)